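; BP_Scene is a Beat Saber scene actor that animates the stage and shifts its lighting between red and blue.
; Five seconds after BeginPlay it plays one-shot animations on the main scene mesh and six music meshes, then starts LightChange.
; LightChange shuffles delay times and flip-flops a timeline forward and backward.
; Timeline updates drive the MP_Alpha collection's LightAlpha and the steam particle color, and re-trigger LightChange to keep cycling.
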(event `self.ReceiveBeginPlay`
  (`KismetSystemLibrary.Delay` 5.0)
  (`SkeletalMeshComponent.PlayAnimation` (`self.ScenesAnimMesh`) "/Game/BeatSaber/Scenes/scene/ScenesAnimMesh_Anim.ScenesAnimMesh_Anim" false)
  (`SkeletalMeshComponent.PlayAnimation` (`self.ScenesAnimMushicMeshR1`) "/Game/BeatSaber/Scenes/ScenesAnimMushicMesh_Anim.ScenesAnimMushicMesh_Anim" false)
  (`SkeletalMeshComponent.PlayAnimation` (`self.ScenesAnimMushicMeshL2`) "/Game/BeatSaber/Scenes/ScenesAnimMushicMesh_Anim.ScenesAnimMushicMesh_Anim" false)
  (`SkeletalMeshComponent.PlayAnimation` (`self.ScenesAnimMushicMeshL3`) "/Game/BeatSaber/Scenes/ScenesAnimMushicMesh_Anim.ScenesAnimMushicMesh_Anim" false)
  (`SkeletalMeshComponent.PlayAnimation` (`self.ScenesAnimMushicMeshR2`) "/Game/BeatSaber/Scenes/ScenesAnimMushicMesh_Anim.ScenesAnimMushicMesh_Anim" false)
  (`SkeletalMeshComponent.PlayAnimation` (`self.ScenesAnimMushicMeshR3`) "/Game/BeatSaber/Scenes/ScenesAnimMushicMesh_Anim.ScenesAnimMushicMesh_Anim" false)
  (`SkeletalMeshComponent.PlayAnimation` (`self.ScenesAnimMushicMeshL1`) "/Game/BeatSaber/Scenes/ScenesAnimMushicMesh_Anim.ScenesAnimMushicMesh_Anim" false)
  (`self.LightChange` :!label _label))

(event `LightChange`
  (bind _chagetime (`self.ChageTime`))
  (`KismetArrayLibrary.Array_Shuffle` _chagetime)
  (for _array_element _chagetime
    (`KismetSystemLibrary.Delay` _array_element)
    (`/Engine/EditorBlueprintResources/StandardMacros.FlipFlop`
      (:`A`
        (bind (_direction _time) (`Timeline|AlphaTime` :!label _label_2)
          (:`Update`
            (`KismetMaterialLibrary.SetScalarParameterValue` "/Game/BeatSaber/Meterials/MP_Alpha.MP_Alpha" "LightAlpha" _time)
            (`FXSystemComponent.SetVectorParameter` (`self.Particle_Steam_Lit`) "color" (`KismetMathLibrary.VLerp` (5.0 0.5 0.5) (0.5 0.5 5.0) _time))
            (goto _label))))
      (:`B`
        (goto _label_2 :!via `Reverse`)))))

(fn `UserConstructionScript`)