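; BP_SaberUI is the Beat Saber game's menu actor, showing Start and Quit elements plus a win or fail window.
; GameWin displays score and max combo and plays a win sound; GameFailed swaps the window to its fail material.
; Both call PlayMusic on the found BP_BoxSpawner, change Start to Restart, and switch the VR pawn's controllers from saber blades to lasers.
; HideUI hides the Start and Quit elements.
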(event `self.ReceiveBeginPlay`
  (bind _outactors (`GameplayStatics.GetAllActorsOfClass` "/Game/BeatSaber/BluePrints/BP_BoxSpawner.BP_BoxSpawner_C"))
  (set `self.RefBP_BoxSpawner` (`|GetArrayItem` _outactors)))

(event `HideUI`
  ;[1 1 1] Hide UI when needed which was uesd in level bp
  (`SceneComponent.SetVisibility` (`self.Quit`) false false)
  (`SceneComponent.SetVisibility` (`self.Start`) false false))

(event `GameWin`
  (params (MaxCombo :type Integer) (Score :type Integer))
  (`|ExecutionSequence`
    (:`then_0`
      (`/Game/BeatSaber/BluePrints/BP_BoxSpawner.PlayMusic` (`self.RefBP_BoxSpawner`))
      ;[1 1 1] Show combo and score
      (`TextRenderComponent.K2_SetText` (`self.Score`) (`KismetTextLibrary.Conv_IntToText` Score))
      (`TextRenderComponent.K2_SetText` (`self.Combo`) (`KismetTextLibrary.Conv_IntToText` MaxCombo))
      (`GameplayStatics.PlaySound2D` "/Game/Win.Win" 1.0 1.0 0.0 null null))
    (:`then_1`
      ;[1 1 1] Show menu and laser when win
      (`PrimitiveComponent.SetMaterial` (`self.Start`) 0 "/Game/BeatSaber/Meterials/M_UI_Restart.M_UI_Restart")
      (`SceneComponent.SetVisibility` (`self.Quit`) true false)
      (`SceneComponent.SetVisibility` (`self.Window`) true false)
      (`SceneComponent.SetVisibility` (`self.Combo`) true false)
      (`SceneComponent.SetVisibility` (`self.Score`) true false)
      (`SceneComponent.SetVisibility` (`self.Start`) true false)
      (bind _asmotion_controller_pawn (cast `/Game/VirtualRealityBP/Blueprints/MotionControllerPawn` (`GameplayStatics.GetPlayerPawn` 0)))
      (`/Game/VirtualRealityBP/Blueprints/MotionControllerPawn.GrabEvent` _asmotion_controller_pawn true)
      (`/Game/VirtualRealityBP/Blueprints/BP_MotionController.LaserVisible` (`/Game/VirtualRealityBP/Blueprints/MotionControllerPawn.LeftController` _asmotion_controller_pawn) false true)
      (`/Game/VirtualRealityBP/Blueprints/BP_MotionController.LaserVisible` (`/Game/VirtualRealityBP/Blueprints/MotionControllerPawn.RightController` _asmotion_controller_pawn) false true))))

(event `GameFailed`
  ;[1 1 1] Show menu and laser when failed
  (`/Game/BeatSaber/BluePrints/BP_BoxSpawner.PlayMusic` (`self.RefBP_BoxSpawner`))
  ;;[1 1 1] Replace start with restart
  (`PrimitiveComponent.SetMaterial` (`self.Start`) 0 "/Game/BeatSaber/Meterials/M_UI_Restart.M_UI_Restart")
  ;;[1 1 1] Replace win with fail
  (`PrimitiveComponent.SetMaterial` (`self.Window`) 0 "/Game/BeatSaber/Meterials/M_window_Fail.M_window_Fail")
  (`SceneComponent.SetVisibility` (`self.Quit`) true false)
  (`SceneComponent.SetVisibility` (`self.Window`) true false)
  (`SceneComponent.SetVisibility` (`self.Start`) true false)
  (bind _asmotion_controller_pawn (cast `/Game/VirtualRealityBP/Blueprints/MotionControllerPawn` (`GameplayStatics.GetPlayerPawn` 0)))
  (`/Game/VirtualRealityBP/Blueprints/MotionControllerPawn.GrabEvent` _asmotion_controller_pawn true)
  (`/Game/VirtualRealityBP/Blueprints/BP_MotionController.LaserVisible` (`/Game/VirtualRealityBP/Blueprints/MotionControllerPawn.LeftController` _asmotion_controller_pawn) false true)
  (`/Game/VirtualRealityBP/Blueprints/BP_MotionController.LaserVisible` (`/Game/VirtualRealityBP/Blueprints/MotionControllerPawn.RightController` _asmotion_controller_pawn) false true))

(fn `UserConstructionScript`)