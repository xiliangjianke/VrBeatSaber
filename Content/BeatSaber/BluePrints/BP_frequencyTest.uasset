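; BP_frequencyTest is a timer test Blueprint that runs a countdown with debug printing.
; Its Construction Script, rather than BeginPlay, starts a looping one-second timer that calls CountDown by function name.
; While Time is above zero, CountDown decrements it and prints the new value and a "Hello" message; the timer is never cleared.
; The event graph holds only empty placeholder events.
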(fn `CountDown`
  (if (> (`self.Time`) 0)
    (bind _output_get (set `self.Time` (- (`self.Time`) 1)))
    (`KismetSystemLibrary.PrintString` (`KismetStringLibrary.Conv_IntToString` _output_get))
    (`KismetSystemLibrary.PrintString` "Hello")))

(fn `UserConstructionScript`
  (`KismetSystemLibrary.K2_SetTimer` null "CountDown" 1.0 true))