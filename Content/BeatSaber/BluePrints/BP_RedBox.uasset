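; BP_RedBox is the red note block in a Beat Saber-style game, animating into place and reacting to cuts.
; BoxAnimation shows the box number and runs a timeline for the initial rush, angle change and drop to one of two ground-collision depths, with impact sparks.
; BoxCutting fires once, removes the four directional colliders, prints score only for an Up cut, then replaces the box with a direction-oriented sliced actor.
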(event `BoxCutting`
  (params (CutDirectionName :type String))
  (bind _ref_sliceboxred (`self.Ref_SliceBoxRed`))
  (bind (_relativerotation_roll _relativerotation_pitch _relativerotation_yaw) (`KismetMathLibrary.BreakRotator` (`SceneComponent.RelativeRotation` (`self.RedBox`))))
  (`/Engine/EditorBlueprintResources/StandardMacros.DoOnce` false
    (:`Completed`
      (set `self.CutDirectionName` CutDirectionName)
      (`ActorComponent.K2_DestroyComponent` (`self.BoxCollionDown`))
      (`ActorComponent.K2_DestroyComponent` (`self.BoxCollionLeft`))
      (`ActorComponent.K2_DestroyComponent` (`self.BoxCollionRight`))
      (`ActorComponent.K2_DestroyComponent` (`self.BoxCollionUp`))
      (switch `string` (`self.CutDirectionName`)
        (:`BoxCollionUp`
          (`KismetSystemLibrary.PrintString` "Get score!")
          (`|SpawnActorFromClass` _ref_sliceboxred (`KismetMathLibrary.MakeTransform` (`self.K2_GetActorLocation`) (* (`SceneComponent.RelativeRotation` (`self.RedBox`)) -1)) "Undefined" "OverrideRootScale" null null :!label _label))
        (:`BoxCollionDown`
          (`KismetSystemLibrary.PrintString` "Failed!")
          (goto _label))
        (:`BoxCollionLeft`
          ;[1 1 1] Chage slice box direction for left and right
          (`KismetSystemLibrary.PrintString` "Failed!" :!label _label_2)
          (`|SpawnActorFromClass` _ref_sliceboxred (`KismetMathLibrary.MakeTransform` (`self.K2_GetActorLocation`) (`KismetMathLibrary.MakeRotator` (* (+ _relativerotation_roll 90.0) -1.0) _relativerotation_pitch _relativerotation_yaw)) "Undefined" "OverrideRootScale" null null))
        (:`BoxCollionRight`
          (goto _label_2)))
      (`self.K2_DestroyActor`))))

(event `BoxAnimation`
  (params (BoxAngle :type "/Game/BeatSaber/BluePrints/EnumBoxAngle Enum" :default "NewEnumerator0") (BoxNum :type Integer) (UpOrDownOfBox :type Boolean))
  (bind (_returnvalue_x _returnvalue_y _returnvalue_z) (`KismetMathLibrary.BreakVector` (`self.K2_GetActorLocation`)))
  (bind _redbox (`self.RedBox`))
  (`|ExecutionSequence`
    (:`then_0`
      ;[1 1 1] Calculate Z distance for collision between box and ground,lower box is -50, higher box is -110
      (if UpOrDownOfBox
        (set `self.DistanceToCollisionGround` -50.0)
        (else
          (set `self.DistanceToCollisionGround` -110.0))))
    (:`then_1`
      (`TextRenderComponent.K2_SetText` (`self.TextRender`) (`KismetTextLibrary.Conv_IntToText` BoxNum))
      (bind (_direction _initialboxaccelerate _collisiontogroundtime _changeangletime) (`Timeline|AnimitionTime`)
        (:`Update`
          ;[1 1 1] Set rotation for animition of changing box angle
          (`SceneComponent.K2_SetRelativeRotation` _redbox (`KismetMathLibrary.RLerp` (struct) (`KismetMathLibrary.MakeRotator` (select `/Game/BeatSaber/BluePrints/EnumBoxAngle` BoxAngle :`NewEnumerator1` -45.0 :`NewEnumerator2` -90.0 :`NewEnumerator3` -135.0 :`NewEnumerator4` 180.0 :`NewEnumerator5` 45.0 :`NewEnumerator6` 90.0 :`NewEnumerator7` 135.0 :!type "Float (single-precision)")) _changeangletime) false false)
          ;[1 1 1] Set location for initial accelarate animation and collision between box and ground animition
          (`SceneComponent.K2_SetRelativeLocation` _redbox (`KismetMathLibrary.MakeVector` (`KismetMathLibrary.Lerp` -2000.0 0.0 _initialboxaccelerate) 0.0 (`KismetMathLibrary.Lerp` 0.0 (`self.DistanceToCollisionGround`) _collisiontogroundtime)) false false))
        (:`LightEvent`
          ;[1 1 1] Spark when box hit ground
          (`GameplayStatics.SpawnEmitterAtLocation` (`self.ParticleOfBoxToGround`) (`KismetMathLibrary.MakeVector` _returnvalue_x _returnvalue_y (+ _returnvalue_z (`self.DistanceToCollisionGround`) 25.0))))))))

(fn `UserConstructionScript`)