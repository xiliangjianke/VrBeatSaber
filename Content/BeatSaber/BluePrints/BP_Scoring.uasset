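; BP_Scoring is the Beat Saber-style game's scoring actor, tracking combo, max combo, score, life and a multiplier.
; Successes raise score, life and a multiplier progress bar, with text displays and the MP_Score parameter collection driving the visuals.
; Failures or Box overlaps reset combo and progress, lower the multiplier, and drain life inversely to it.
; BP_SaberUI receives victory results, or the failure call after the game pauses on depleted life.
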(event `ComboSuccess`
  (bind _lifeincrement (`self.LifeIncrement`))
  (`|ExecutionSequence`
    (:`then_0`
      ;[1 1 1] Combo and score up
      (bind _output_get (set `self.Combo` (+ (`self.Combo`) 1)))
      (`self.GetMaxCombo`)
      (`TextRenderComponent.K2_SetText` (`self.Comb`) (`KismetTextLibrary.Conv_IntToText` _output_get))
      (bind _output_get_2 (set `self.TotalScore` (+ (`self.TotalScore`) 10)))
      (`TextRenderComponent.K2_SetText` (`self.Score`) (`KismetTextLibrary.Conv_IntToText` _output_get_2)))
    (:`then_1`
      ;[1 1 1] HP bar 1 increase
      (if (< (`self.Life`) 1.0)
        (bind _output_get_3 (set `self.Life` (+ (`self.Life`) 0.05)))
        (`KismetMaterialLibrary.SetScalarParameterValue` "/Game/BeatSaber/Meterials/MP_Score.MP_Score" "HpBar2" _output_get_3)))
    (:`then_2`
      ;[1 1 1] Hp bar 2
      (if (< _lifeincrement 8)
        (bind _output_get_4 (set `self.LifrParaIncre` (+ (`self.LifrParaIncre`) (/ 1.0 (`KismetMathLibrary.Conv_IntToDouble` _lifeincrement)))))
        (`KismetMaterialLibrary.SetScalarParameterValue` "/Game/BeatSaber/Meterials/MP_Score.MP_Score" "HpBar1" _output_get_4)
        (if (>= _output_get_4 1.0)
          (bind _output_get_5 (set `self.LifeIncrement` (+ 1 (`self.LifeIncrement`))))
          (`TextRenderComponent.K2_SetText` (`self.HpBarMultiply`) (`KismetTextLibrary.Conv_IntToText` _output_get_5))
          (`KismetSystemLibrary.Delay` 0.5)
          (bind _output_get_6 (set `self.LifrParaIncre` 0.0))
          (`KismetMaterialLibrary.SetScalarParameterValue` "/Game/BeatSaber/Meterials/MP_Score.MP_Score" "HpBar1" _output_get_6))))))

(event `self.ReceiveBeginPlay`
  (bind _outactors (`GameplayStatics.GetAllActorsOfClass` "/Game/BeatSaber/BluePrints/BP_SaberUI.BP_SaberUI_C"))
  (set `self.RefBP_SaberUI` (`|GetArrayItem` _outactors)))

(event `GameVictory`
  (`/Game/BeatSaber/BluePrints/BP_SaberUI.GameWin` (`self.RefBP_SaberUI`) (`self.MaxCombo`) (`self.TotalScore`)))

(event `GetMaxCombo`
  (bind _combo (`self.Combo`))
  ;[1 1 1] Get max combo for win menu
  (if (< (`self.MaxCombo`) _combo)
    (set `self.MaxCombo` _combo)))

(event `ComboFailed`
  (bind _lifeincrement (`self.LifeIncrement`))
  (bind _life (`self.Life`))
  (`|ExecutionSequence` :!label _label
    (:`then_0`
      ;[1 1 1] Clear combo and HP bar2
      (`self.GetMaxCombo`)
      (bind _output_get (set `self.Combo` 0))
      (`TextRenderComponent.K2_SetText` (`self.Comb`) (`KismetTextLibrary.Conv_IntToText` _output_get))
      (bind _output_get_2 (set `self.LifrParaIncre` 0.0))
      (`KismetMaterialLibrary.SetScalarParameterValue` "/Game/BeatSaber/Meterials/MP_Score.MP_Score" "HpBar1" _output_get_2))
    (:`then_1`
      ;[1 1 1] Clear HpBarMultiply
      (if (> _lifeincrement 1)
        (bind _output_get_3 (set `self.LifeIncrement` (- _lifeincrement 1)))
        (`TextRenderComponent.K2_SetText` (`self.HpBarMultiply`) (`KismetTextLibrary.Conv_IntToText` _output_get_3))))
    (:`then_2`
      ;[1 1 1] decrease HP
      (if (<= _life 0.0)
        (`GameplayStatics.SetGamePaused` true)
        (`/Game/BeatSaber/BluePrints/BP_SaberUI.GameFailed` (`self.RefBP_SaberUI`))
        (else
          (bind _output_get_4 (set `self.Life` (- _life (* (/ 1.0 (`KismetMathLibrary.Conv_IntToDouble` (`self.LifeIncrement`))) 0.1))))
          (`KismetMaterialLibrary.SetScalarParameterValue` "/Game/BeatSaber/Meterials/MP_Score.MP_Score" "HpBar2" _output_get_4))))))

(event `self.Box.OnComponentBeginOverlap`
  (params (OverlappedComponent :type "PrimitiveComponent Object Reference") (OtherActor :type "Actor Object Reference") (OtherComp :type "PrimitiveComponent Object Reference") (OtherBodyIndex :type Integer) (bFromSweep :type Boolean) (SweepResult :type "HitResult Structure (by ref)"))
  (goto _label))

(fn `UserConstructionScript`)